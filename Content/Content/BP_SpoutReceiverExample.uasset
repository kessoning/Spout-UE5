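; BP_SpoutReceiverExample is an example actor that receives a Spout video stream and displays it on its Visualizer mesh.
; BeginPlay creates a dynamic instance of the unlit display material on the Visualizer.
; Each Tick receives the named Spout source into that material and an optional render target, with optional async receive, raising a HasSignal parameter on success.
; EndPlay closes the receiver.
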(event EventBeginPlay
  ;[1 1 1] Comment
  (bind _returnvalue (Rendering|Material|CreateDynamicMaterialInstance (Variables|Default|GetVisualizer) 0 "/SpoutPlugin/Content/M_SpoutDisplayUnlit.M_SpoutDisplayUnlit" "None" :!class /Script/Engine.PrimitiveComponent))
  (Variables|Default|SetSpoutConsumerMaterial _returnvalue))

(event EventTick
  (params (DeltaSeconds :type Float%20%28single-precision%29))
  (bind (_outtexture _returnvalue) (Class|SpoutBPFunctionLibrary|SpoutReceiverwithMaterial (Variables|Spout|GetSpoutName) (Variables|Default|GetSpoutConsumerMaterial) "None" (Variables|Spout|GetOutputRenderTarget) "Auto" (Variables|Spout|GetAsyncReceiveBeta)))
  (Variables|Default|SetSpoutReceivedTexture _outtexture)
  (if _returnvalue
    (Rendering|Material|SetScalarParameterValue (Variables|Default|GetSpoutConsumerMaterial) "HasSignal" 1.0 :!class /Script/Engine.MaterialInstanceDynamic)))

(event EventEndPlay
  (params (EndPlayReason :type EEndPlayReason%20Enum :default "Destroyed"))
  (Class|SpoutBPFunctionLibrary|CloseReceiver (Variables|Spout|GetSpoutName) (Variables|Default|GetSpoutReceivedTexture) (Variables|Default|GetSpoutConsumerMaterial)))

(fn ConstructionScript)